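; BP_Equipmentbox is an interactable equipment box actor that opens and closes an equipment container UI.
; On BeginPlay it creates and stores a UI_EQBContainer widget.
; Interact toggles that widget in the viewport, switching the first player controller between Game-and-UI input with a visible cursor and Game-only input without one.
; It always reports itself as interactable, and its interaction-info request returns nothing custom.
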(event EventBeginPlay
  (bind _returnvalue (UserInterface|CreateWidget "/Game/UI/EquipmentBox/UI_EQBContainer.UI_EQBContainer_C"))
  (Variables|Default|SetUI _returnvalue))

(event Collision|EventActorBeginOverlap
  (params (OtherActor :type Actor%20Object%20Reference)))

(event EventTick
  (params (DeltaSeconds :type Float%20%28single-precision%29)))

(event EventInteract
  (params (InteractionInstigator :type Actor%20Object%20Reference))
  (bind _returnvalue (Game|GetPlayerController 0))
  (bind _ui (Variables|Default|GetUI))
  (if (UserInterface|Viewport|IsinViewport (Variables|Default|GetUI))
    (Widget|RemovefromParent _ui)
    (Input|SetInputModeGameOnly _returnvalue)
    (Variables|/Script/Engine.PlayerController|SetbShowMouseCursor _returnvalue false)
    (else
      (UserInterface|Viewport|AddtoViewport _ui 1)
      (Input|SetInputModeGameandUI _returnvalue _ui "DoNotLock" false)
      (Variables|/Script/Engine.PlayerController|SetbShowMouseCursor _returnvalue true))))

(fn ConstructionScript)

(fn CheckIsInteractable
  (params (InteractionInstigator :type Actor%20Object%20Reference))
  (return true))

(fn RequestInteractionInfo
  (params (InteractionInstigator :type Actor%20Object%20Reference))
  (return ""))