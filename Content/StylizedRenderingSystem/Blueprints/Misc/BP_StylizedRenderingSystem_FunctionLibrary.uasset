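; Blueprint function library for the Stylized Rendering System that gives access to the light color manager.
; Get Light Manager fetches the manager by sending a message to the Game State.
; RegisterLightColor and UnregisterLightColor forward a color or an ID to that manager and return its result.
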(fn GetLightManager
  (bind _light_color_manager (Class|BPCelShadedLightManagerInterface|GetLightColorManager(Message) (Game|GetGameState)))
  (return _light_color_manager))

(fn RegisterLightColor
  (params (Color :type Linear%20Color%20Structure))
  (bind _id (Default|RegisterLightColor (CallFunction|GetLightManager) Color))
  (return _id))

(fn UnregisterLightColor
  (params (ID :type Integer%20%28by%20ref%29))
  (bind _successful (Default|UnregisterLightColor (CallFunction|GetLightManager) ID))
  (return _successful))