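; BP_WallHitState is a character state for a wall hit, suspending gravity while the character reacts.
; On enter it zeroes the CharacterMovementComponent's gravity scale and plays a montage on the context's skeletal mesh.
; When the montage completes, it fires the EventBus hit delegate with the DamageInfo held in cross-state data.
; On exit it sets gravity scale back to normal.
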(event EventOnStateEnter
  (bind _statescomp (Variables|Default|GetStatesComp))
  (bind _compcontext (Variables|/Script/ProjectGrivenka.BaseContextableComponent|GetCompContext _statescomp))
  (bind _ascharacter_movement_component (Utilities|Casting|CastToCharacterMovementComponent (Variables|/Script/ProjectGrivenka.ContextSystem|GetMovementComp _compcontext)))
  (Variables|/Script/Engine.CharacterMovementComponent|SetGravityScale _ascharacter_movement_component 0.0)
  (Animation|Montage|PlayMontage (Variables|/Script/ProjectGrivenka.ContextSystem|GetSkeletalMeshComp _compcontext) (Variables|Default|GetMentalMontage)
    (:OnCompleted
      (Default|CallHitDelegate (Variables|/Script/ProjectGrivenka.ContextSystem|GetEventBus _compcontext) 0 (.damageinfo (Variables|/Script/ProjectGrivenka.CharacterStatesSystem|GetCrossStateData (Variables|Default|GetStatesComp)))))))

(event EventOnStateExit
  (Variables|/Script/Engine.CharacterMovementComponent|SetGravityScale (stale EventOnStateEnter _ascharacter_movement_component) 1.0))