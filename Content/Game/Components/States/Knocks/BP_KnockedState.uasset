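; Knocked state for a states component that defines which knockback data a character uses for each hit direction.
; On Init it calls the parent, then builds the KnockbackData map from ten directions to containers with Standing, FarPush and Launch sets.
; Standing uses directional light sets, with some directions sharing one.
; FarPush and Launch share one explosive set per direction, drawn from only Top, Bottom and Front variants.
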(event EventInit
  (params (InStatesComp :type Character%20States%20System%20Object%20Reference))
  (bind _bottomexplosiveset (Variables|Default|GetBottomExplosiveSet))
  (bind _frontexplosiveset (Variables|Default|GetFrontExplosiveSet))
  (bind _frontexplosiveset_2 (Variables|Default|GetFrontExplosiveSet))
  (bind _frontexplosiveset_3 (Variables|Default|GetFrontExplosiveSet))
  (bind _bottomexplosiveset_2 (Variables|Default|GetBottomExplosiveSet))
  (bind _topexplosiveset (Variables|Default|GetTopExplosiveSet))
  (bind _topexplosiveset_2 (Variables|Default|GetTopExplosiveSet))
  (bind _topexplosiveset_3 (Variables|Default|GetTopExplosiveSet))
  (bind _bottomexplosiveset_3 (Variables|Default|GetBottomExplosiveSet))
  (bind _bottomexplosiveset_4 (Variables|Default|GetBottomExplosiveSet))
  (|CallParentFunction InStatesComp)
  (Variables|Default|SetKnockbackData (Utilities|Map|MakeMap "TOP" (Utilities|Struct|MakeKnockBackDataContainer (Variables|Default|GetTopLightSet) _topexplosiveset _topexplosiveset) "TOPLEFT" (Utilities|Struct|MakeKnockBackDataContainer (Variables|Default|GetLeftLightSet) _topexplosiveset_2 _topexplosiveset_2) "TOPRIGHT" (Utilities|Struct|MakeKnockBackDataContainer (Variables|Default|GetRightLightSet) _topexplosiveset_3 _topexplosiveset_3) "BOTTOM" (Utilities|Struct|MakeKnockBackDataContainer (Variables|Default|GetBottomRightLightSet) _bottomexplosiveset_4 _bottomexplosiveset_4) "BOTTOMLEFT" (Utilities|Struct|MakeKnockBackDataContainer (Variables|Default|GetBottomLeftLightSet) _bottomexplosiveset _bottomexplosiveset) "BOTTOMRIGHT" (Utilities|Struct|MakeKnockBackDataContainer (Variables|Default|GetBottomRightLightSet) _bottomexplosiveset_3 _bottomexplosiveset_3) "LEFT" (Utilities|Struct|MakeKnockBackDataContainer (Variables|Default|GetLeftLightSet) _frontexplosiveset_2 _frontexplosiveset_2) "RIGHT" (Utilities|Struct|MakeKnockBackDataContainer (Variables|Default|GetRightLightSet) _frontexplosiveset _frontexplosiveset) "FRONT" (Utilities|Struct|MakeKnockBackDataContainer (Variables|Default|GetTopLightSet) _frontexplosiveset_3 _frontexplosiveset_3) "BACK" (Utilities|Struct|MakeKnockBackDataContainer (Variables|Default|GetBackLightSet) _bottomexplosiveset_2 _bottomexplosiveset_2))))