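; Modular appearance component that builds a character's body from appearance, equipment and gender data.
; LoadAppearance sets the part meshes, then applies shape-key morph targets to the main mesh and every part.
; It then merges the part mesh assets into one skeletal mesh, placed on the Torso component and unhidden.
; Finally, the main skeletal mesh component takes Torso as its master pose component.
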(event EventLoadAppearance
  (params (InAppearance :type Persisted%20Character%20Appearance%20Structure) (InEquipments :type Persisted%20Equipments%20Structure) (InGender :type Integer))
  (Class|ModularAppearanceSystem|SetModularPartsMeshes InAppearance InEquipments InGender)
  (CallFunction|ProcessMorphTargets (.ShapeKeyValues (Utilities|Struct|BreakPersistedCharacterAppearance InAppearance)))
  (CallFunction|MergeBodyMesh)
  (CallFunction|SetupMasterPose))

(fn ApplyMorphTargets
  (params (Mesh :type Skeletal%20Mesh%20Component%20Object%20Reference) (TargetMap :type Map%20of%20Names%20to%20Float%20%28single-precision%29s) (IsBaked :type Boolean))
  (bind _output_get (LocalVariables|SetMorphTargets TargetMap))
  (bind _keys (Utilities|Map|Keys _output_get))
  (for _array_element _keys
    (Components|SkeletalMesh|SetMorphTarget Mesh _array_element (.Value (Utilities|Map|Find (LocalVariables|GetMorphTargets) _array_element)) true)
    (if IsBaked
      _)))

(fn ProcessMorphTargets
  (params (MorphTargets :type Map%20of%20Names%20to%20Float%20%28single-precision%29s))
  (bind _modularparts (Variables|Default|GetModularParts))
  (CallFunction|ApplyMorphTargets (Variables|/Script/ProjectGrivenka.ContextSystem|GetSkeletalMeshComp (Variables|Default|GetCompContext)) MorphTargets true)
  (CallFunction|ApplyMorphTargets (.hair _modularparts) MorphTargets true)
  (CallFunction|ApplyMorphTargets (.headwear _modularparts) MorphTargets true)
  (CallFunction|ApplyMorphTargets (.facialhair _modularparts) MorphTargets true)
  (CallFunction|ApplyMorphTargets (.outertorso _modularparts) MorphTargets true)
  (CallFunction|ApplyMorphTargets (.torso _modularparts) MorphTargets true)
  (CallFunction|ApplyMorphTargets (.legs _modularparts) MorphTargets true)
  (CallFunction|ApplyMorphTargets (.hands _modularparts) MorphTargets true)
  (CallFunction|ApplyMorphTargets (.feet _modularparts) MorphTargets true)
  (CallFunction|ApplyMorphTargets (.acc1 _modularparts) MorphTargets true)
  (CallFunction|ApplyMorphTargets (.acc2 _modularparts) MorphTargets true)
  (CallFunction|ApplyMorphTargets (.acc3 _modularparts) MorphTargets true))

(fn SetupMasterPose
  (Class|SkinnedMeshComponent|SetMasterPoseComponent (Variables|/Script/ProjectGrivenka.ContextSystem|GetSkeletalMeshComp (Variables|Default|GetCompContext)) (.torso (Variables|Default|GetModularParts)) false))

(fn MergeBodyMesh
  (bind _modularparts (Variables|Default|GetModularParts))
  (bind _modularparts_2 (Variables|Default|GetModularParts))
  (bind _returnvalue (Class|ModularAppearanceSystem|MergeMeshes (Utilities|Struct|MakeSkeletalMeshMergeParams 0 0 (Utilities|Array|MakeArray (Variables|/Script/Engine.SkinnedMeshComponent|GetSkeletalMesh (.hair _modularparts)) (Variables|/Script/Engine.SkinnedMeshComponent|GetSkeletalMesh (.headwear _modularparts)) (Variables|/Script/Engine.SkinnedMeshComponent|GetSkeletalMesh (.facialhair _modularparts)) (Variables|/Script/Engine.SkinnedMeshComponent|GetSkeletalMesh (.outertorso _modularparts)) (Variables|/Script/Engine.SkinnedMeshComponent|GetSkeletalMesh (.torso _modularparts)) (Variables|/Script/Engine.SkinnedMeshComponent|GetSkeletalMesh (.legs _modularparts)) (Variables|/Script/Engine.SkinnedMeshComponent|GetSkeletalMesh (.hands _modularparts)) (Variables|/Script/Engine.SkinnedMeshComponent|GetSkeletalMesh (.feet _modularparts)) (Variables|/Script/Engine.SkinnedMeshComponent|GetSkeletalMesh (.acc1 _modularparts)) (Variables|/Script/Engine.SkinnedMeshComponent|GetSkeletalMesh (.acc2 _modularparts)) (Variables|/Script/Engine.SkinnedMeshComponent|GetSkeletalMesh (.acc3 _modularparts))) 0 false false 0)))
  (Class|SkinnedMeshComponent|SetSkeletalMesh (.torso _modularparts_2) _returnvalue true)
  (Development|SetHiddeninGame (.torso _modularparts_2) false false))