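; BP_Lootables is an interactable world actor that can be looted.
; On BeginPlay it initializes its interaction context and fills the text of its widget component.
; Interact calls forward to the interact system component, whose OnInteract event triggers the loot system's OnLooted with the instigator.
; It always reports itself interactable and requests a one-off, non-latent interaction with a bend-over floor pickup montage.
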(event OnInteract(BP_InteractSystem)
  (params (InteractInstigator :type Actor%20Object%20Reference))
  (Class|LootSystem|OnLooted (Variables|Default|GetBP_LootSystem) InteractInstigator))

(event EventBeginPlay
  (CallFunction|InitializeContext (Variables|Default|GetCtx) 0 0 0 0 self)
  (bind _astext (Utilities|Casting|CastToText (UserInterface|GetUserWidgetObject (Variables|Default|GetWidget))))
  (Variables|/Game/UI/Text.Text_C|SetText _astext (Variables|Default|GetTExt)))

(event EventInteract
  (params (InteractionInstigator :type Actor%20Object%20Reference))
  (Class|InteractSystem|Interact (Variables|Default|GetBP_InteractSystem) InteractionInstigator))

(fn ConstructionScript)

(fn CheckIsInteractable
  (params (InteractionInstigator :type Actor%20Object%20Reference))
  (return true))

(fn GetContext
  (return (Variables|Default|GetCtx)))

(fn GetInteractableItem
  (bind _returnvalue (Class|InteractSystem|GetInteractableItem (Variables|Default|GetBP_InteractSystem)))
  (return _returnvalue))

(fn GetInteractionCollider
  (return 0))

(fn GetInteractSystemComp
  (return (Variables|Default|GetBP_InteractSystem)))

(fn RequestInteractionInfo
  (params (InteractionInstigator :type Actor%20Object%20Reference))
  (return (Utilities|Struct|MakeInteractionInfo false 0.0 "/Game/Mannequin/Animations/Placeholders/Loot/Loot_FloorPickUp_BendOver_RightHand_Montage.Loot_FloorPickUp_BendOver_RightHand_Montage" "INL_NORMAL" "INU_ONEOFF")))