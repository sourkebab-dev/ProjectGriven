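; BP_BaseGoons is a base goon NPC character that wires shared context, persistence and modular appearance systems together.
; On BeginPlay it initializes a context with its mesh, movement, anim instance, controller and self, exposed through GetContext.
; Save and load calls forward to the persistence and modular appearance components, with leftover debug prints in LoadAppearance.
; GetModularParts is an empty stub.
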(event EventBeginPlay
  (bind _mesh (Variables|Character|GetMesh))
  (CallFunction|InitializeContext (Variables|Default|GetCtx) _mesh (Variables|Character|GetCharacterMovement) (Components|SkeletalMesh|GetAnimInstance _mesh) (Pawn|GetController) self))

(event EventLoadPersistance
  (params (InCharacterData :type Persisted%20Character%20Data%20Structure))
  (Class|CharacterPersistanceSystem|LoadData (Variables|Default|GetBP_PersistanceSystem)))

(event EventLoadAppearance
  (params (InAppearance :type Persisted%20Character%20Appearance%20Structure) (InEquipments :type Persisted%20Equipments%20Structure) (InGender :type Integer))
  (Development|PrintString "eafafawfawf")
  (Development|PrintString (Utilities|String|Append (Utilities|GetDisplayName (Variables|/Script/ProjectGrivenka.BaseContextableComponent|GetCompContext (Variables|Default|GetBP_ModularAppearanceSystem))) "tete"))
  (Class|ModularAppearanceSystem|LoadAppearance (Variables|Default|GetBP_ModularAppearanceSystem) InAppearance InEquipments InGender))

(event EventSaveAppearance
  (params (InAppearance :type Persisted%20Character%20Appearance%20Structure) (InEquipments :type Persisted%20Equipments%20Structure) (InGender :type Integer))
  (Class|ModularAppearanceSystem|SaveAppearance (Variables|Default|GetBP_ModularAppearanceSystem) InAppearance InEquipments InGender))

(fn ConstructionScript
  (|CallParentFunction))

(fn GetContext
  (return (Variables|Default|GetCtx)))

(fn GetModularParts
  (return ""))

(fn SavePersistance
  (bind _outcharacterdata (Class|CharacterPersistanceSystem|SaveData (Variables|Default|GetBP_PersistanceSystem)))
  (return _outcharacterdata))