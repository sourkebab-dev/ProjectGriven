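; Base ally grunt NPC character that combines RPG and equipment components with an AI-driven combat context.
; On BeginPlay it initializes the context from its mesh, movement and anim instance, sets up the AI context and equips a hardcoded common katana.
; Interface events and functions are thin pass-throughs: attributes and effects go to BPRPGSystem, while weapons, attacks and blocking go to BPEquipmentSystem.
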(event EventBeginPlay
  (bind _mesh (Variables|Character|GetMesh))
  ;[1 1 1] Setup
  (CallFunction|InitializeContext (Variables|Default|GetContext) _mesh (Variables|Character|GetCharacterMovement) (Components|SkeletalMesh|GetAnimInstance _mesh) 0 self)
  (CallFunction|AIContextInitiation (AI|GetAIController self))
  (Class|EquipmentSystem|LoadEquipments (Variables|Default|GetBP_EquipmentSystem) (Utilities|Struct|MakePersistedEquipments (Utilities|Struct|MakePersistedEquipmentItem "00000000000000000000000000000000" "Katana_Common"))))

(event EventInitEffectFortitudeDamage
  (params (EffectInstigator :type Actor%20Object%20Reference) (InDamageInfo :type Damage%20Info%20Structure))
  ;[1 1 1] RPG Sys Imp
  (Class|CharacterSystem|InitEffectForitudeDamage (Variables|Default|GetBP_RPGSystem) EffectInstigator InDamageInfo))

(event EventLoadEquipments
  (params (InEquipments :type Persisted%20Equipments%20Structure))
  ;[1 1 1] Equipment Sys Impl
  (Class|EquipmentSystem|LoadEquipments (Variables|Default|GetBP_EquipmentSystem) InEquipments))

(event EventDisableWeaponDamageColliders
  ;[1 1 1] Equipment Sys Impl
  (Class|EquipmentSystem|DisableWeaponDamageColliders (Variables|Default|GetBP_EquipmentSystem)))

(event EventRemoveEffectbyTag
  (params (EffectTag :type Gameplay%20Tag%20Structure))
  ;[1 1 1] RPG Sys Imp
  (Class|CharacterSystem|RemoveEffectsbyTag (Variables|Default|GetBP_RPGSystem) EffectTag false))

(event EventLoadAttributes
  (params (InAttributes :type Persisted%20Attributes%20Structure))
  ;[1 1 1] RPG Sys Imp
  (Class|CharacterSystem|InitializeAttributes (Variables|Default|GetBP_RPGSystem) InAttributes))

(event EventInitEffectReceiveHit
  (params (EffectInstigator :type Actor%20Object%20Reference) (InDamageInfo :type Damage%20Info%20Structure))
  ;[1 1 1] RPG Sys Imp
  (Class|CharacterSystem|InitEffectReceiveHit (Variables|Default|GetBP_RPGSystem) EffectInstigator InDamageInfo))

(event EventInitEffectDepleteStamina
  (params (EffectInstigator :type Actor%20Object%20Reference) (InValue :type Float%20%28single-precision%29))
  ;[1 1 1] RPG Sys Imp
  (Class|CharacterSystem|InitEffectDepleteStamina (Variables|Default|GetBP_RPGSystem) EffectInstigator InValue))

(event EventInitEffectbyRegenName
  (params (EffectInstigator :type Actor%20Object%20Reference) (InPrefabName :type Name :default "None"))
  ;[1 1 1] RPG Sys Imp
  (Class|CharacterSystem|InitEffectbyRegenName (Variables|Default|GetBP_RPGSystem) EffectInstigator InPrefabName))

(event EventInitEffectbyPrefabName
  (params (EffectInstigator :type Actor%20Object%20Reference) (InPrefabName :type Name :default "None") (InOverrideValue :type Float%20%28single-precision%29) (IsValueOverridden :type Boolean))
  ;[1 1 1] RPG Sys Imp
  (Class|CharacterSystem|InitEffectbyPrefabName (Variables|Default|GetBP_RPGSystem) EffectInstigator InPrefabName InOverrideValue IsValueOverridden))

(event EventInitEffectbyPrefab
  (params (EffectInstigator :type Actor%20Object%20Reference) (InEffectPrefab :type Effect%20Prefab%20Object%20Reference) (InOverrideValue :type Float%20%28single-precision%29) (IsValueOverridden :type Boolean))
  ;[1 1 1] RPG Sys Imp
  (Class|CharacterSystem|InitEffectbyPrefab (Variables|Default|GetBP_RPGSystem) EffectInstigator InEffectPrefab InOverrideValue IsValueOverridden))

(fn ConstructionScript)

(fn GetAttributeCurrentValue
  (params (InAttributeCode :type EAttributeCode%20Enum :default "ATT_Health"))
  (bind _returnvalue (Class|CharacterSystem|GetAttributeCurrentValue (Variables|Default|GetBP_RPGSystem) InAttributeCode))
  (return _returnvalue))

(fn GetAttributeMaxValue
  (params (InAttributeCode :type EAttributeCode%20Enum :default "ATT_Health"))
  (bind _returnvalue (Class|CharacterSystem|GetAttributeMaxValue (Variables|Default|GetBP_RPGSystem) InAttributeCode))
  (return _returnvalue))

(fn GetBlockInfo
  (bind (_outblockinfo _outdamageabsorption) (Class|EquipmentSystem|GetBlockInfo (Variables|Default|GetBP_EquipmentSystem)))
  (return _outblockinfo _outdamageabsorption))

(fn GetCharacterSystemComp
  (return (Variables|Default|GetBP_RPGSystem)))

(fn GetContext
  (return (Variables|Default|GetContext)))

(fn GetCurrentAttackStaminaUsage
  (params (InCurrentAttackValues :type Attack%20Values%20Structure))
  (bind _returnvalue (Class|EquipmentSystem|CalculateAttackStaminaCost (Variables|Default|GetBP_EquipmentSystem) InCurrentAttackValues))
  (return _returnvalue))

(fn GetEquipmentSystemComp
  (return (Variables|Default|GetBP_EquipmentSystem)))

(fn GetNextMainAttack
  (params (InMovementType :type EAttackMovementType%20Enum :default "AM_DEFAULT") (InCurrentAttackValues :type Attack%20Values%20Structure))
  (bind _returnvalue (Class|EquipmentSystem|GetNextAttackValue (Variables|Default|GetBP_EquipmentSystem) InMovementType InCurrentAttackValues))
  (return _returnvalue))