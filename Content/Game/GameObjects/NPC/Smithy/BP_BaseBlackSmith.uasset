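; Base blacksmith NPC that the player can interact with to start dialogue and that handles smithing requests.
; On BeginPlay it fills a shared context with its mesh, movement, animation instance and controller.
; Interaction is always allowed and passes to the interact component, whose OnInteract event starts default dialogue, while smith requests forward to the smith component.
; Getters expose these parts, and interaction info specifies a one-off, movement-blocking action with an animation.
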(event OnInteract(BP_InteractSystem)
  (params (InteractInstigator :type Actor%20Object%20Reference))
  (Class|DialogueSystem|StartDefaultDialogue (Variables|Default|GetBP_DialogueSystem)))

(event EventBeginPlay
  (bind _mesh (Variables|Character|GetMesh))
  (CallFunction|InitializeContext (Variables|Default|GetCtx) _mesh (Variables|Character|GetCharacterMovement) (Components|SkeletalMesh|GetAnimInstance _mesh) (Pawn|GetController) self))

(event EventSmithRequest
  (Class|SmithSystem|OnReceiveSmithRequest (Variables|Default|GetBP_SmithSystem)))

(event EventInteract
  (params (InteractionInstigator :type Actor%20Object%20Reference))
  (Class|InteractSystem|Interact (Variables|Default|GetBP_InteractSystem) InteractionInstigator))

(fn ConstructionScript)

(fn CheckIsInteractable
  (params (InteractionInstigator :type Actor%20Object%20Reference))
  (return true))

(fn GetContext
  (return (Variables|Default|GetCtx)))

(fn GetDialogueSystemComp
  (return (Variables|Default|GetBP_DialogueSystem)))

(fn GetInteractableItem
  (bind _returnvalue (Class|InteractSystem|GetInteractableItem (Variables|Default|GetBP_InteractSystem)))
  (return _returnvalue))

(fn GetInteractionCollider
  (return (Variables|Default|GetBox)))

(fn GetInteractSystemComp
  (return (Variables|Default|GetBP_InteractSystem)))

(fn RequestInteractionInfo
  (params (InteractionInstigator :type Actor%20Object%20Reference))
  (return (Utilities|Struct|MakeInteractionInfo false 0.0 "/Game/Mannequin/Animations/Placeholders/Mage/RaiseAmp.RaiseAmp" "INL_BLOCK" "INU_ONEOFF")))