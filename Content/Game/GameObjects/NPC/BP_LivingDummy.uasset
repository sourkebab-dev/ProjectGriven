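; BP_LivingDummy is an NPC dummy character that exposes RPG attribute, effect, hostility and AI command functions.
; On BeginPlay it initializes its context from its mesh, movement component, anim instance and controller.
; It acts as a thin forwarding layer: attribute and effect calls go to BPRPGSystem, while commands and hostility checks go to BPAIContextSystem.
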(event EventBeginPlay
  (bind _mesh (Variables|Character|GetMesh))
  (CallFunction|InitializeContext (Variables|Default|Getctx) _mesh (Variables|Character|GetCharacterMovement) (Components|SkeletalMesh|GetAnimInstance _mesh) (Pawn|GetController) self))

(event EventInitEffectbyRegenName
  (params (EffectInstigator :type Actor%20Object%20Reference) (InPrefabName :type Name :default "None"))
  (Class|CharacterSystem|InitEffectbyRegenName (Variables|Default|GetBP_RPGSystem) EffectInstigator InPrefabName))

(event EventInitEffectbyPrefabName
  (params (EffectInstigator :type Actor%20Object%20Reference) (InPrefabName :type Name :default "None") (InOverrideValue :type Float%20%28single-precision%29) (IsValueOverridden :type Boolean))
  (Class|CharacterSystem|InitEffectbyPrefabName (Variables|Default|GetBP_RPGSystem) EffectInstigator InPrefabName InOverrideValue IsValueOverridden))

(event EventInitEffectbyPrefab
  (params (EffectInstigator :type Actor%20Object%20Reference) (InEffectPrefab :type Effect%20Prefab%20Object%20Reference) (InOverrideValue :type Float%20%28single-precision%29) (IsValueOverridden :type Boolean))
  (Class|CharacterSystem|InitEffectbyPrefab (Variables|Default|GetBP_RPGSystem) EffectInstigator InEffectPrefab InOverrideValue IsValueOverridden))

(event EventSignalCommandtoArea
  (params (CommandInfo :type Command%20Info%20Structure))
  (Class|AIContextSystem|SignalCommandtoArea (Variables|Default|GetBP_AIContextSystem) CommandInfo))

(event EventSignalCommandtoActor
  (params (CommandReceiveActor :type Actor%20Object%20Reference) (CommandInfo :type Command%20Info%20Structure))
  (Class|AIContextSystem|SignalCommandtoActor (Variables|Default|GetBP_AIContextSystem) CommandReceiveActor CommandInfo))

(event EventOnCommanded
  (params (CommandInstigator :type Actor%20Object%20Reference) (CommandInfo :type Command%20Info%20Structure))
  (Class|AIContextSystem|OnCommanded (Variables|Default|GetBP_AIContextSystem) CommandInstigator CommandInfo))

(event EventUnSubscribeAttributeChanges
  (params (InAttributeCode :type EAttributeCode%20Enum :default "ATT_Health") (InDelegate :type Delegate%20%28by%20ref%29))
  (Class|CharacterSystem|UnSubscribeAttributeChanges (Variables|Default|GetBP_RPGSystem) InAttributeCode InDelegate))

(event EventSubscribeAttributeChanges
  (params (InAttributeCode :type EAttributeCode%20Enum :default "ATT_Health") (InDelegate :type Delegate%20%28by%20ref%29))
  (Class|CharacterSystem|SubscribeAttributeChanges (Variables|Default|GetBP_RPGSystem) InAttributeCode InDelegate))

(event EventRemoveEffectbyTag
  (params (EffectTag :type Gameplay%20Tag%20Structure))
  (Class|CharacterSystem|RemoveEffectsbyTag (Variables|Default|GetBP_RPGSystem) EffectTag false))

(event EventLoadAttributes
  (params (InAttributes :type Persisted%20Attributes%20Structure))
  (Class|CharacterSystem|InitializeAttributes (Variables|Default|GetBP_RPGSystem) InAttributes))

(event EventInitEffectReceiveHit
  (params (EffectInstigator :type Actor%20Object%20Reference) (InDamageInfo :type Damage%20Info%20Structure))
  (Class|CharacterSystem|InitEffectReceiveHit (Variables|Default|GetBP_RPGSystem) EffectInstigator InDamageInfo))

(event EventInitEffectFortitudeDamage
  (params (EffectInstigator :type Actor%20Object%20Reference) (InDamageInfo :type Damage%20Info%20Structure))
  (Class|CharacterSystem|InitEffectForitudeDamage (Variables|Default|GetBP_RPGSystem) EffectInstigator InDamageInfo))

(event EventInitEffectDepleteStamina
  (params (EffectInstigator :type Actor%20Object%20Reference) (InValue :type Float%20%28single-precision%29))
  (Class|CharacterSystem|InitEffectDepleteStamina (Variables|Default|GetBP_RPGSystem) EffectInstigator InValue))

(fn ConstructionScript)

(fn CheckHostility
  (params (ToCheckActor :type Actor%20Object%20Reference))
  (bind _returnvalue (Class|AIContextSystem|CheckHostility (Variables|Default|GetBP_AIContextSystem) ToCheckActor))
  (return _returnvalue))

(fn GetAttributeCurrentValue
  (params (InAttributeCode :type EAttributeCode%20Enum :default "ATT_Health"))
  (bind _returnvalue (Class|CharacterSystem|GetAttributeCurrentValue (Variables|Default|GetBP_RPGSystem) InAttributeCode))
  (return _returnvalue))

(fn GetAttributeMaxValue
  (params (InAttributeCode :type EAttributeCode%20Enum :default "ATT_Health"))
  (bind _returnvalue (Class|CharacterSystem|GetAttributeMaxValue (Variables|Default|GetBP_RPGSystem) InAttributeCode))
  (return _returnvalue))

(fn GetCharacterSystemComp
  (return (Variables|Default|GetBP_RPGSystem)))

(fn GetContext
  (return (Variables|Default|Getctx)))

(fn GetHostilityType
  (return (Variables|/Script/ProjectGrivenka.AIContextSystem|GetHostilityType (Variables|Default|GetBP_AIContextSystem))))