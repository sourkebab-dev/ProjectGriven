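; Player spawn point that brings the first two crew members into the level and gives control to the first.
; On BeginPlay it spawns them from the game instance's Crew data, the first as the player and the second as an NPC.
; Possession waits for the player's ContextAvailable mounted callback, which unsubscribes itself, has player controller 0 possess the pawn, then loads the in-game UI through UIManager.
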(event Custom|OnCharacterMounted
  ;[1 1 1] Spawn
  (Class|ContextAvailable|UnsubtoMountedFunction (stale EventBeginPlay _ascontext_available) (delegate Custom|OnCharacterMounted))
  (bind _aspawn (Utilities|Casting|CastToPawn (stale EventBeginPlay _returnvalue)))
  (Pawn|Possess (Game|GetPlayerController 0) _aspawn)
  (bind _asbp_base_game_instance (Utilities|Casting|CastToBP_BaseGameInstance (Game|GetGameInstance)))
  (Class|UIManager|LoadinGameUI (Variables|/Script/ProjectGrivenka.BaseGameInstance|GetUIManager _asbp_base_game_instance)))

(event EventBeginPlay
  ;[1 1 1] Spawn
  (bind _asbp_base_game_instance (Utilities|Casting|CastToBP_BaseGameInstance (Game|GetGameInstance)))
  (bind _returnvalue (Class|PlayerSpawnPoint|SpawnPlayer (Utilities|Array|Get(acopy) (Variables|/Script/ProjectGrivenka.BaseGameInstance|GetCrew _asbp_base_game_instance)) false))
  (bind _ascontext_available (Utilities|Casting|CastToContextAvailable _returnvalue))
  (Class|ContextAvailable|SubscribetoMountedFunction _ascontext_available (delegate Custom|OnCharacterMounted))
  (Class|PlayerSpawnPoint|SpawnPlayer (Utilities|Array|Get(acopy) (Variables|/Script/ProjectGrivenka.BaseGameInstance|GetCrew _asbp_base_game_instance) 1) true))

(fn ConstructionScript)