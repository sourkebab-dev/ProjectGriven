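; BP_SpawnPoint is a spawn point actor that creates a BP_ControllableCharacter when a character's spawner dispatcher fires.
; On BeginPlay it finds the first existing controllable character and binds SpawnThing to that dispatcher.
; SpawnThing spawns a character at the point's XY with Z zeroed, then offset by 100 on each axis.
; The new character loads the first Crew entry from BP_BaseGameInstance.
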(event Custom|Spawn%20Thing
  (bind _returnvalue (Transformation|GetActorLocation))
  (bind _returnvalue_2 (Game|SpawnActorfromClass "/Game/ThirdPersonCPP/Blueprints/BP_ControllableCharacter.BP_ControllableCharacter_C" (Math|Transform|MakeTransform (+ (Math|Vector|MakeVector (.x _returnvalue) (.y _returnvalue) 0.0) 1e+02)) "Undefined" 0 0))
  (bind _asbp_base_game_instance (Utilities|Casting|CastToBP_BaseGameInstance (Game|GetGameInstance)))
  (Class|BaseCharacter|LoadData _returnvalue_2 (Utilities|Array|Get(acopy) (Variables|/Script/ProjectGrivenka.BaseGameInstance|GetCrew _asbp_base_game_instance))))

(event EventBeginPlay
  (bind _outactors (Actor|GetAllActorsOfClass "/Game/ThirdPersonCPP/Blueprints/BP_ControllableCharacter.BP_ControllableCharacter_C"))
  (Utilities|IsValid (Utilities|Array|Get(acopy) _outactors)
    (:Is%20Valid
      (EventDispatchers|BindEventtoSpawnerDispatcher (Utilities|Array|Get(acopy) _outactors) (delegate Custom|Spawn%20Thing)))))

(event Collision|EventActorBeginOverlap
  (params (OtherActor :type Actor%20Object%20Reference)))

(event EventTick
  (params (DeltaSeconds :type Float%20%28single-precision%29)))

(fn ConstructionScript)