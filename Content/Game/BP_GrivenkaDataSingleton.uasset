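; Data singleton for the Grivenka game that serves character appearance data from DataTables.
; Getter functions look up wearable info, body info, skin color, body type data and morph group values by ID, each from its own table.
; Body type lookups first translate the type ID to a row name through the BodyTypeKey map, and morph group lookups return only the morph values from the row.
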(fn GetWearableInfo
  (params (WearableId :type Name :default "None"))
  (bind _returnvalue (Utilities|GetDataTableRow (Variables|SingletonData|GetWearableData) WearableId)
    (:then
      (return (Utilities|Struct|BreakDT_STR_WearableInfo _returnvalue)))
    (:RowNotFound
      (return ""))))

(fn GetBodyInfo
  (params (BodyId :type Name :default "None"))
  (bind _returnvalue (Utilities|GetDataTableRow (Variables|SingletonData|GetBodyData) BodyId)
    (:then
      (return (Utilities|Struct|BreakDT_STR_BodyInfo _returnvalue)))
    (:RowNotFound
      (return ""))))

(fn GetSkinColor
  (params (SkinColorId :type Name :default "None"))
  (bind _returnvalue (Utilities|GetDataTableRow (Variables|SingletonData|GetSkinColorData) SkinColorId)
    (:then
      (return (Utilities|Struct|BreakDT_STR_SkinColor _returnvalue)))))

(fn GetBodyTypeData
  (params (TypeId :type Integer))
  (bind _returnvalue (Utilities|GetDataTableRow (Variables|SingletonData|GetBodyTypeData) (.Value (Utilities|Map|Find (LocalVariables|GetBodyTypeKey) TypeId)))
    (:then
      (return (Utilities|Struct|BreakDT_STR_BodyTypeData _returnvalue)))))

(fn GetMorphGroupValues
  (params (MorphGroupId :type Name :default "None"))
  (bind _returnvalue (Utilities|GetDataTableRow (Variables|SingletonData|GetMorphGroupData) MorphGroupId)
    (:then
      (return (.morphvalues (Utilities|Struct|BreakDT_STR_MorphData _returnvalue))))))